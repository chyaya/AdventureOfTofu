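; Game mode for the Tofu game that builds a sector-based level when play begins.
; On BeginPlay, its level generator component generates a 5x5 level from the current position, then MoveSector loads that starting sector.
; MoveSector looks up the sector class at the given coordinates and spawns it at the world origin, without removing earlier sectors or updating the current position.
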(event `self.ReceiveBeginPlay`
  (`LevelGeneratorCompo.GenerateLevel` (`self.BP_LevelGeneratorCompo`) 5 5 (`self.CurrentPosX`) (`self.CurrentPosY`))
  (`self.MoveSector` (`self.CurrentPosX`) (`self.CurrentPosY`)))

(fn `MoveSector`
  (params (x :type Integer) (y :type Integer))
  (bind _returnvalue (`LevelGeneratorCompo.GetSector` (`self.BP_LevelGeneratorCompo`) x y))
  (`|SpawnActorFromClass` _returnvalue (`KismetMathLibrary.MakeTransform` (0.0 0.0 0.0)) "Undefined" "OverrideRootScale" null null))

(fn `UserConstructionScript`)